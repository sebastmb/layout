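; Base sword Blueprint that the player can pick up and use for light and heavy combo attacks against enemies.
; An overlap sphere toggles the prompt widget and input; interacting gives the player a sword if none is held, then destroys this actor.
; Attack events step through montage arrays using the character's chain counters, calling empty combo hooks.
; HitEvent damages each hit EnemyParent_BP once via an already-damaged list, boosting heavy hits; AttackTrace is empty.
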(event `HitEvent`
  (params (Damage :type "Float (double-precision)") (Hit :type "HitResult Structure"))
  (bind _characterref (`self.CharacterRef`))
  (set `self.Damage` Damage)
  (bind _outactors (`GameplayStatics.GetAllActorsOfClass` "/Game/Actores/EnemigoPirata/Blueprints/Enemys/EnemyParent_BP.EnemyParent_BP_C"))
  (for _array_element _outactors
    (set `self.DamageEnemy` _array_element)
    (if (and (== _array_element (`.HitActor` (`GameplayStatics.BreakHitResult` Hit))) (not (`KismetArrayLibrary.Array_Contains` (`self.AlreadyDamageEnemy`) (`self.DamageEnemy`))))
      (`KismetArrayLibrary.Array_Add` (`self.AlreadyDamageEnemy`) (`self.DamageEnemy`))
      (if (`/Game/Actores/EnemigoPirata/Blueprints/Character/PlayerCharacter.LightAttack` _characterref)
        (`/Game/Actores/EnemigoPirata/Blueprints/Enemys/HealthDamageInterface.DealingDamage` (`self.DamageEnemy`) (`self.Damage`) (`self.CharacterRef`))
        (elif (`/Game/Actores/EnemigoPirata/Blueprints/Character/PlayerCharacter.HeavyAttack` _characterref)
          (`/Game/Actores/EnemigoPirata/Blueprints/Enemys/HealthDamageInterface.DealingDamage` (`self.DamageEnemy`) (+ (`self.Damage`) (* (`self.Damage`) 0.5)) (`self.CharacterRef`)))))))

(event `self.Sphere.OnComponentBeginOverlap`
  (params (OverlappedComponent :type "PrimitiveComponent Object Reference") (OtherActor :type "Actor Object Reference") (OtherComp :type "PrimitiveComponent Object Reference") (OtherBodyIndex :type Integer) (bFromSweep :type Boolean) (SweepResult :type "HitResult Structure (by ref)"))
  ;[1 1 1] Can player pick up?
  (cast `/Game/Actores/EnemigoPirata/Blueprints/Character/PlayerCharacter` OtherActor)
  (`self.EnableInput` (`GameplayStatics.GetPlayerController` 0))
  (`SceneComponent.SetVisibility` (`self.Widget`) true false))

(event `self.Sphere.OnComponentEndOverlap`
  (params (OverlappedComponent :type "PrimitiveComponent Object Reference") (OtherActor :type "Actor Object Reference") (OtherComp :type "PrimitiveComponent Object Reference") (OtherBodyIndex :type Integer))
  ;[1 1 1] Can player pick up?
  (cast `/Game/Actores/EnemigoPirata/Blueprints/Character/PlayerCharacter` OtherActor)
  (`self.DisableInput` (`GameplayStatics.GetPlayerController` 0))
  (`SceneComponent.SetVisibility` (`self.Widget`) false false))

(event `InputAction|Interect`
  (params (Key :type "Key Structure"))
  (bind _asplayer_character (cast `/Game/Actores/EnemigoPirata/Blueprints/Character/PlayerCharacter` (`GameplayStatics.GetPlayerCharacter` 0) :!pure true))
  ;[1 1 1] Pickup
  (:`Pressed`
    (if (not (`KismetSystemLibrary.IsValid` (`/Game/Actores/EnemigoPirata/Blueprints/Character/PlayerCharacter.SwordRef` _asplayer_character)))
      (`/Game/Actores/EnemigoPirata/Blueprints/Character/PlayerCharacter.PickupSword` _asplayer_character)
      (`self.K2_DestroyActor`))))

(event `self.ReceiveBeginPlay`
  ;[1 1 1] Char ref
  (bind _asplayer_character (cast `/Game/Actores/EnemigoPirata/Blueprints/Character/PlayerCharacter` (`GameplayStatics.GetPlayerCharacter` 0)))
  (set `self.CharacterRef` _asplayer_character))

(event `LightAttack`
  (bind _characterref (`self.CharacterRef`))
  (bind _characterref_2 (`self.CharacterRef`))
  (bind _chainlightattack (`/Game/Actores/EnemigoPirata/Blueprints/Character/PlayerCharacter.ChainLightAttack` (`self.CharacterRef`)))
  (bind _output (`|GetArrayItem` (`self.LightAttacks`) (`/Game/Actores/EnemigoPirata/Blueprints/Character/PlayerCharacter.ChainLightAttack` _characterref_2)))
  (if (== (+ (`/Game/Actores/EnemigoPirata/Blueprints/Character/PlayerCharacter.ChainLightAttack` (`self.CharacterRef`)) 1) (`KismetArrayLibrary.Array_Length` (`self.LightAttacks`)))
    (set `/Game/Actores/EnemigoPirata/Blueprints/Character/PlayerCharacter.LastAttack` true _characterref))
  (switch `int` (`/Game/Actores/EnemigoPirata/Blueprints/Character/PlayerCharacter.ChainLightAttack` _characterref)
    (:`0`
      (`Character.PlayAnimMontage` _characterref_2 _output 1.2 "None")
      (`self.ComboLightAttack` _chainlightattack)
      (set `/Game/Actores/EnemigoPirata/Blueprints/Character/PlayerCharacter.ChainLightAttack` 1 (`self.CharacterRef`)))
    (:`1`
      (`Character.PlayAnimMontage` _characterref_2 _output 1.2 "None")
      (`self.ComboLightAttack` _chainlightattack)
      (set `/Game/Actores/EnemigoPirata/Blueprints/Character/PlayerCharacter.ChainLightAttack` 2 (`self.CharacterRef`)))
    (:`2`
      (`Character.PlayAnimMontage` _characterref_2 _output 1.2 "None")
      (`self.ComboLightAttack` _chainlightattack)
      (set `/Game/Actores/EnemigoPirata/Blueprints/Character/PlayerCharacter.ChainLightAttack` 3 (`self.CharacterRef`)))
    (:`3`
      (`Character.PlayAnimMontage` _characterref_2 _output 1.2 "None")
      (`self.ComboLightAttack` _chainlightattack)
      (set `/Game/Actores/EnemigoPirata/Blueprints/Character/PlayerCharacter.ChainLightAttack` 0 (`self.CharacterRef`)))))

(event `HeavyAttack`
  (bind _characterref (`self.CharacterRef`))
  (bind _characterref_2 (`self.CharacterRef`))
  (bind _chainheavyattack (`/Game/Actores/EnemigoPirata/Blueprints/Character/PlayerCharacter.ChainHeavyAttack` (`self.CharacterRef`)))
  (bind _output (`|GetArrayItem` (`self.HeavyAttacks`) (`/Game/Actores/EnemigoPirata/Blueprints/Character/PlayerCharacter.ChainHeavyAttack` _characterref_2)))
  (if (== (+ (`/Game/Actores/EnemigoPirata/Blueprints/Character/PlayerCharacter.ChainHeavyAttack` (`self.CharacterRef`)) 1) (`KismetArrayLibrary.Array_Length` (`self.HeavyAttacks`)))
    (set `/Game/Actores/EnemigoPirata/Blueprints/Character/PlayerCharacter.LastAttack` true _characterref))
  (switch `int` (`/Game/Actores/EnemigoPirata/Blueprints/Character/PlayerCharacter.ChainHeavyAttack` _characterref)
    (:`0`
      (`Character.PlayAnimMontage` _characterref_2 _output 1.0 "None")
      (`self.ComboHeavyAttack` _chainheavyattack)
      (set `/Game/Actores/EnemigoPirata/Blueprints/Character/PlayerCharacter.ChainHeavyAttack` 1 (`self.CharacterRef`)))
    (:`1`
      (`Character.PlayAnimMontage` _characterref_2 _output 1.0 "None")
      (`self.ComboHeavyAttack` _chainheavyattack)
      (set `/Game/Actores/EnemigoPirata/Blueprints/Character/PlayerCharacter.ChainHeavyAttack` 2 (`self.CharacterRef`)))
    (:`2`
      (`Character.PlayAnimMontage` _characterref_2 _output 1.0 "None")
      (`self.ComboHeavyAttack` _chainheavyattack)
      (set `/Game/Actores/EnemigoPirata/Blueprints/Character/PlayerCharacter.ChainHeavyAttack` 3 (`self.CharacterRef`)))
    (:`3`
      (`Character.PlayAnimMontage` _characterref_2 _output 1.0 "None")
      (`self.ComboHeavyAttack` _chainheavyattack)
      (set `/Game/Actores/EnemigoPirata/Blueprints/Character/PlayerCharacter.ChainHeavyAttack` 0 (`self.CharacterRef`)))))

(event `ComboLightAttack`
  (params (ChainLightAttack :type Integer)))

(event `ComboHeavyAttack`
  (params (ChainHeavyAttack :type Integer)))

(fn `AttackTrace`)

(fn `UserConstructionScript`)
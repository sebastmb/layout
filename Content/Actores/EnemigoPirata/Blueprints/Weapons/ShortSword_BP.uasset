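; Short sword weapon Blueprint in the pirate enemy folder, handling combo chaining and melee hit detection for its owning character.
; Light and heavy combo events copy their first two chain steps into the opposite attack's counter on the character.
; AttackTrace casts short complex line traces backward from twelve collision points, targeting Pawns except the owner.
; Each successful trace passes the weapon's damage and hit result to HitEvent.
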(event `ComboLightAttack_1`
  (params (ChainLightAttack :type Integer))
  (bind _characterref (`self.CharacterRef`))
  (switch `int` ChainLightAttack
    (:`0`
      (set `/Game/Actores/EnemigoPirata/Blueprints/Character/PlayerCharacter.ChainHeavyAttack` 0 _characterref))
    (:`1`
      (set `/Game/Actores/EnemigoPirata/Blueprints/Character/PlayerCharacter.ChainHeavyAttack` 1 _characterref))))

(event `ComboHeavyAttack_1`
  (params (ChainHeavyAttack :type Integer))
  (bind _characterref (`self.CharacterRef`))
  (switch `int` ChainHeavyAttack
    (:`0`
      (set `/Game/Actores/EnemigoPirata/Blueprints/Character/PlayerCharacter.ChainLightAttack` 0 _characterref))
    (:`1`
      (set `/Game/Actores/EnemigoPirata/Blueprints/Character/PlayerCharacter.ChainLightAttack` 1 _characterref))))

(event `self.AttackTrace`
  (for _array_element (`|MakeArray` (`self.Collision1`) (`self.Collision2`) (`self.Collision3`) (`self.Collision4`) (`self.Collision5`) (`self.Collision6`) (`self.Collision7`) (`self.Collision8`) (`self.Collision9`) (`self.Collision10`) (`self.Collision11`) (`self.Collision12`))
    (bind _returnvalue (`SceneComponent.K2_GetComponentLocation` _array_element))
    (bind (_outhit _returnvalue_2) (`KismetSystemLibrary.LineTraceSingleForObjects` _returnvalue (- _returnvalue (* (`KismetMathLibrary.GetForwardVector` (`SceneComponent.K2_GetComponentRotation` _array_element)) 10.0)) (`|MakeArray` "ObjectTypeQuery3" :!type "EObjectTypeQuery Enum") true (`|MakeArray` (`self.CharacterRef`) :!type "Actor Object Reference") "None" true (struct :`R` 1.0 :`A` 1.0) (struct :`G` 1.0 :`A` 1.0) 0.2))
    (if _returnvalue_2
      (`self.HitEvent` (`self.Damage`) _outhit))))

(fn `UserConstructionScript`
  (`parent.UserConstructionScript`))
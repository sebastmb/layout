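; Enemy sword Blueprint that damages the player's Mayla character during attacks.
; The EnemyAttackTrace event casts a short Pawn line trace from its Box component, opposite the box's forward vector, ignoring all EnemyParent_BP actors.
; Any hit applies a small fixed damage to player character 0, cast to Mayla_CharacterBP, rather than to the traced actor.
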(event `self.ReceiveBeginPlay`)

(event `self.ReceiveTick`
  (params (DeltaSeconds :type "Float (single-precision)")))

(event `EnemyAttackTrace`
  (for _array_element (`|MakeArray` (`self.Box`))
    (bind _outactors (`GameplayStatics.GetAllActorsOfClass` "/Game/Actores/EnemigoPirata/Blueprints/Enemys/EnemyParent_BP.EnemyParent_BP_C"))
    (bind _returnvalue (`SceneComponent.K2_GetComponentLocation` _array_element))
    (bind (_outhit _returnvalue_2) (`KismetSystemLibrary.LineTraceSingleForObjects` _returnvalue (- _returnvalue (* (`KismetMathLibrary.GetForwardVector` (`SceneComponent.K2_GetComponentRotation` _array_element)) 10.0)) (`|MakeArray` "ObjectTypeQuery3" :!type "EObjectTypeQuery Enum") true _outactors "None" true (struct :`R` 1.0 :`A` 1.0) (struct :`G` 1.0 :`A` 1.0) 0.2))
    (if _returnvalue_2
      (bind _asmayla_character_bp (cast `/Game/Actores/Personaje/Mayla/Mayla_CharacterBP` (`GameplayStatics.GetPlayerCharacter` 0)))
      (`GameplayStatics.ApplyDamage` _asmayla_character_bp 0.005))))

(fn `UserConstructionScript`)
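; Health component, named for a mage enemy, that sets health to maximum on BeginPlay and handles incoming damage.
; TakeDamage applies only while the player's CanRoll is true, and lethal hits set IsDead and fire the death dispatcher.
; Non-lethal hits raise a hurt-animation flag for two seconds, call PlayAnimMontage on the player character, then call the player's ChainAttacks.
; Both outcomes print debug text.
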(event `self.ReceiveBeginPlay`
  (`self.intHealth`))

(event `TakeDamage`
  (params (DamageAmount :type "Float (double-precision)"))
  (bind _returnvalue (- (`self.CurrentHealth`) DamageAmount))
  (bind _asplayer_character (cast `/Game/Actores/EnemigoPirata/Blueprints/Character/PlayerCharacter` (`GameplayStatics.GetPlayerCharacter` 0) :!pure true))
  (if (`/Game/Actores/EnemigoPirata/Blueprints/Character/PlayerCharacter.CanRoll?` _asplayer_character)
    (if (>= DamageAmount (`self.CurrentHealth`))
      (set `self.CurrentHealth` _returnvalue)
      (set `self.isDead` true)
      (`KismetSystemLibrary.PrintString` "DEAD")
      (`self.DeathDispatcher`)
      (else
        (bind _output_get (set `self.CurrentHealth` _returnvalue))
        (`KismetSystemLibrary.PrintString` (`KismetStringLibrary.Conv_DoubleToString` _output_get))
        (set `self.TakeDamageAnim` true)
        (`Character.PlayAnimMontage` _asplayer_character null 1.0 "None")
        (`KismetSystemLibrary.Delay` 2.0)
        (set `self.TakeDamageAnim` false)
        (`/Game/Actores/EnemigoPirata/Blueprints/Character/PlayerCharacter.ChainAttacks` _asplayer_character)))))

(fn `intHealth`
  (set `self.CurrentHealth` (`self.MaxHealth`))
  (set `self.isDead` false))
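; ProceduralWater is a Blueprint that lays out a flat grid of mesh tiles, presumably a water surface going by its name.
; The Construction Script sizes and fills the TipoMesh array from MaxX and MaxY, using it only as a tile counter.
; Each index becomes an InstancedStaticMesh instance, placed by integer division and modulo on MaxY and spaced by TamañoMesh.
; The event graph has no active logic.
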(fn `UserConstructionScript`
  (bind _maxy (`self.MaxY`))
  (bind `_tamañomesh` (`self.TamañoMesh`))
  (bind _returnvalue (- (* (`self.MaxX`) (`self.MaxY`)) 1))
  (`KismetArrayLibrary.Array_Resize` (`self.TipoMesh`) _returnvalue)
  (for _index (range (+ _returnvalue 1))
    (`KismetArrayLibrary.Array_Set` (`self.TipoMesh`) _index))
  (for (_ _array_index) (`self.TipoMesh`)
    (`InstancedStaticMeshComponent.AddInstance` (`self.InstancedStaticMesh`) (`KismetMathLibrary.Conv_VectorToTransform` (`KismetMathLibrary.MakeVector` (`KismetMathLibrary.Conv_IntToDouble` (* (/ _array_index _maxy) `_tamañomesh`)) (`KismetMathLibrary.Conv_IntToDouble` (* `_tamañomesh` (mod _array_index _maxy))))))))
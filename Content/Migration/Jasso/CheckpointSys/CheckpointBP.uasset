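; Checkpoint actor that saves the Mayla player character's location to the "Check" save slot when its sphere is overlapped.
; With its Load flag true, it captures the location, then updates or creates a SaveGameClass object storing that location and Load as true.
; With the flag false, it only rewrites the existing save's Load to false.
; The overlapping actor is not checked, and debug prints report checkpoint activity.
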(event `self.Sphere.OnComponentBeginOverlap`
  (params (OverlappedComponent :type "PrimitiveComponent Object Reference") (OtherActor :type "Actor Object Reference") (OtherComp :type "PrimitiveComponent Object Reference") (OtherBodyIndex :type Integer) (bFromSweep :type Boolean) (SweepResult :type "HitResult Structure (by ref)"))
  (if (`self.Load?`)
    (`|ExecutionSequence`
      (:`then_0`
        (bind _asmayla_character_bp (cast `/Game/Actores/Personaje/Mayla/Mayla_CharacterBP` (`GameplayStatics.GetPlayerCharacter` 0)))
        (set `self.PlayerLocation` (`self.K2_GetActorLocation` _asmayla_character_bp))
        (`KismetSystemLibrary.PrintString` "Checkoint"))
      (:`then_1`
        (bind _returnvalue (`GameplayStatics.DoesSaveGameExist` "Check"))
        (if _returnvalue
          (bind _returnvalue_2 (`GameplayStatics.LoadGameFromSlot` "Check"))
          (bind _assave_game_class (cast `/Game/Migration/Jasso/CheckpointSys/SaveGameClass` _returnvalue_2))
          (set `/Game/Migration/Jasso/CheckpointSys/SaveGameClass.PlayerLocation` (`self.PlayerLocation`) _assave_game_class)
          (set `/Game/Migration/Jasso/CheckpointSys/SaveGameClass.Load?` true _assave_game_class)
          (`GameplayStatics.SaveGameToSlot` _assave_game_class "Check")
          (else
            (bind _returnvalue_3 (`GameplayStatics.CreateSaveGameObject` "/Game/Migration/Jasso/CheckpointSys/SaveGameClass.SaveGameClass_C"))
            (set `/Game/Migration/Jasso/CheckpointSys/SaveGameClass.PlayerLocation` (`self.PlayerLocation`) _returnvalue_3)
            (set `/Game/Migration/Jasso/CheckpointSys/SaveGameClass.Load?` true _returnvalue_3)
            (`GameplayStatics.SaveGameToSlot` _returnvalue_3 "Check")))))
    (else
      (bind _returnvalue_4 (`GameplayStatics.LoadGameFromSlot` "Check"))
      (bind _assave_game_class_2 (cast `/Game/Migration/Jasso/CheckpointSys/SaveGameClass` _returnvalue_4))
      (set `/Game/Migration/Jasso/CheckpointSys/SaveGameClass.Load?` false _assave_game_class_2)
      (`GameplayStatics.SaveGameToSlot` _assave_game_class_2 "Check")
      (`KismetSystemLibrary.PrintString` "Checkpoint Updated"))))

(fn `UserConstructionScript`)